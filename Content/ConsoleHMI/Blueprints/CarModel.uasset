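; CarModel is the 3D car actor that animates its hood, trunk and four doors to mirror the vehicle state on InstrumentCluster_CppBP.
; Tick polls each state flag, using paired DoOnce gates that reset each other so open or close events fire only on changes.
; Each event stops the opposite Timeline and plays its own, lerping a pivot arrow from its current transform toward hard-coded targets.
; Sunroof events are empty, their Timeline logic left disconnected.
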(event Custom|Open%20SunRoof
  ;[0.6158 1 0.9872 1 72] Car SunRoof Anim
)

(event Custom|Close%20SunRoof
  ;[0.6158 1 0.9872 1 72] Car SunRoof Anim
)

(event Custom|Close%20Rear%20Right%20Door
  (bind _rear_right_door_pivot_arrow (Variables|Default|GetRear_right_door_pivot_arrow))
  (bind _rear_right_door_pivot_arrow_2 (Variables|Default|GetRear_right_door_pivot_arrow))
  ;[0.614 1 0.9801 1 72] Car Rear Right Door Anim
  (Utilities|FlowControl|Sequence
    (:then_0
      (bind _open_front_left_door_interpolation_track (Timeline|Timeline_3 Stop)
        (:Update
          (Transformation|SetRelativeLocationAndRotation _rear_right_door_pivot_arrow (Math|Vector|Lerp(Vector) (Variables|/Script/Engine.SceneComponent|GetRelativeLocation _rear_right_door_pivot_arrow) "166.000000,-513.000000,96.000000" _open_front_left_door_interpolation_track) (Math|Rotator|Lerp(Rotator) (Variables|/Script/Engine.SceneComponent|GetRelativeRotation _rear_right_door_pivot_arrow) "0.000000,-48.000000,0.000000" _open_front_left_door_interpolation_track) false false))))
    (:then_1
      (bind _close_front_left_door_interpolation_track (Timeline|Timeline_4 PlayFromStart)
        (:Update
          (Transformation|SetRelativeLocationAndRotation _rear_right_door_pivot_arrow_2 (Math|Vector|Lerp(Vector) (Variables|/Script/Engine.SceneComponent|GetRelativeLocation _rear_right_door_pivot_arrow_2) "166.000000,-513.000000,96.000000" _close_front_left_door_interpolation_track) (Math|Rotator|Lerp(Rotator) (Variables|/Script/Engine.SceneComponent|GetRelativeRotation _rear_right_door_pivot_arrow_2) "0, 0, 0" _close_front_left_door_interpolation_track) false false))))))

(event Custom|Close%20Front%20Left%20Door
  (bind _front_left_door_pivot_arrow (Variables|Default|GetFront_left_door_pivot_arrow))
  (bind _front_left_door_pivot_arrow_2 (Variables|Default|GetFront_left_door_pivot_arrow))
  ;[0.6928 1 0.9815 1 72] Car Front Left Door Anim
  (Utilities|FlowControl|Sequence
    (:then_0
      (bind _open_front_left_door_interpolation_track (Timeline|Open%20Front%20Left%20Door%20Timeline Stop)
        (:Update
          (Transformation|SetRelativeLocationAndRotation _front_left_door_pivot_arrow (Math|Vector|Lerp(Vector) (Variables|/Script/Engine.SceneComponent|GetRelativeLocation _front_left_door_pivot_arrow) "64.000000,-360.000000,89.000000" _open_front_left_door_interpolation_track) (Math|Rotator|Lerp(Rotator) (Variables|/Script/Engine.SceneComponent|GetRelativeRotation _front_left_door_pivot_arrow) "0.000000,48.000000,0.000000" _open_front_left_door_interpolation_track) false false))))
    (:then_1
      (bind _close_front_left_door_interpolation_track (Timeline|Close%20Front%20Left%20Door%20Timeline PlayFromStart)
        (:Update
          (Transformation|SetRelativeLocationAndRotation _front_left_door_pivot_arrow_2 (Math|Vector|Lerp(Vector) (Variables|/Script/Engine.SceneComponent|GetRelativeLocation _front_left_door_pivot_arrow_2) "64.000000,-360.000000,89.000000" _close_front_left_door_interpolation_track) (Math|Rotator|Lerp(Rotator) (Variables|/Script/Engine.SceneComponent|GetRelativeRotation _front_left_door_pivot_arrow_2) "0, 0, 0" _close_front_left_door_interpolation_track) false false))))))

(event Custom|Open%20Rear%20Left%20Door
  (bind _rear_left_door_pivot_arrow (Variables|Default|GetRear_left_door_pivot_arrow))
  (bind _rear_left_door_pivot_arrow_2 (Variables|Default|GetRear_left_door_pivot_arrow))
  ;[0.6135 1 0.9096 1 72] Car Rear Left Door Anim
  (Utilities|FlowControl|Sequence
    (:then_0
      (bind _close_front_left_door_interpolation_track (Timeline|Timeline_2 Stop)
        (:Update
          (Transformation|SetRelativeLocationAndRotation _rear_left_door_pivot_arrow_2 (Math|Vector|Lerp(Vector) (Variables|/Script/Engine.SceneComponent|GetRelativeLocation _rear_left_door_pivot_arrow_2) "166.000000,-362.000000,94.000000" _close_front_left_door_interpolation_track) (Math|Rotator|Lerp(Rotator) (Variables|/Script/Engine.SceneComponent|GetRelativeRotation _rear_left_door_pivot_arrow_2) "0, 0, 0" _close_front_left_door_interpolation_track) false false))))
    (:then_1
      (bind _open_front_left_door_interpolation_track (Timeline|Timeline_1 PlayFromStart)
        (:Update
          (Transformation|SetRelativeLocationAndRotation _rear_left_door_pivot_arrow (Math|Vector|Lerp(Vector) (Variables|/Script/Engine.SceneComponent|GetRelativeLocation _rear_left_door_pivot_arrow) "166.000000,-362.000000,94.000000" _open_front_left_door_interpolation_track) (Math|Rotator|Lerp(Rotator) (Variables|/Script/Engine.SceneComponent|GetRelativeRotation _rear_left_door_pivot_arrow) "0.000000,48.000000,0.000000" _open_front_left_door_interpolation_track) false false))))))

(event Custom|Close%20Rear%20Left%20Door
  (bind _rear_left_door_pivot_arrow (Variables|Default|GetRear_left_door_pivot_arrow))
  (bind _rear_left_door_pivot_arrow_2 (Variables|Default|GetRear_left_door_pivot_arrow))
  ;[0.6135 1 0.9096 1 72] Car Rear Left Door Anim
  (Utilities|FlowControl|Sequence
    (:then_0
      (bind _open_front_left_door_interpolation_track (Timeline|Timeline_1 Stop)
        (:Update
          (Transformation|SetRelativeLocationAndRotation _rear_left_door_pivot_arrow (Math|Vector|Lerp(Vector) (Variables|/Script/Engine.SceneComponent|GetRelativeLocation _rear_left_door_pivot_arrow) "166.000000,-362.000000,94.000000" _open_front_left_door_interpolation_track) (Math|Rotator|Lerp(Rotator) (Variables|/Script/Engine.SceneComponent|GetRelativeRotation _rear_left_door_pivot_arrow) "0.000000,48.000000,0.000000" _open_front_left_door_interpolation_track) false false))))
    (:then_1
      (bind _close_front_left_door_interpolation_track (Timeline|Timeline_2 PlayFromStart)
        (:Update
          (Transformation|SetRelativeLocationAndRotation _rear_left_door_pivot_arrow_2 (Math|Vector|Lerp(Vector) (Variables|/Script/Engine.SceneComponent|GetRelativeLocation _rear_left_door_pivot_arrow_2) "166.000000,-362.000000,94.000000" _close_front_left_door_interpolation_track) (Math|Rotator|Lerp(Rotator) (Variables|/Script/Engine.SceneComponent|GetRelativeRotation _rear_left_door_pivot_arrow_2) "0, 0, 0" _close_front_left_door_interpolation_track) false false))))))

(event Custom|Open%20Hood
  (bind _hood_arrow (Variables|Default|GetHood_arrow))
  (bind _hood_arrow_2 (Variables|Default|GetHood_arrow))
  ;[0.5922 1 0.9929 1 72] Car Hood Anim
  (Utilities|FlowControl|Sequence
    (:then_0
      (bind _close_hood_interpolation_track (Timeline|Close%20Hood%20Interpolation%20Timeline Stop)
        (:Update
          (Transformation|SetRelativeLocationAndRotation _hood_arrow (Math|Vector|Lerp(Vector) (Variables|/Script/Engine.SceneComponent|GetRelativeLocation _hood_arrow) "24.000000,-436.000000,102.000000" _close_hood_interpolation_track) (Math|Rotator|Lerp(Rotator) (Variables|/Script/Engine.SceneComponent|GetRelativeRotation _hood_arrow) "0, 0, 0" _close_hood_interpolation_track) false false))))
    (:then_1
      (bind _open_hood_interpolation_track (Timeline|Open%20Hood%20Interpolation%20Timeline PlayFromStart)
        (:Update
          (Transformation|SetRelativeLocationAndRotation _hood_arrow_2 (Math|Vector|Lerp(Vector) (Variables|/Script/Engine.SceneComponent|GetRelativeLocation _hood_arrow_2) "24.000000,-436.000000,102.000000" _open_hood_interpolation_track) (Math|Rotator|Lerp(Rotator) (Variables|/Script/Engine.SceneComponent|GetRelativeRotation _hood_arrow_2) "-45.000000, 0,0.000000" _open_hood_interpolation_track) false false))))))

(event Custom|Close%20Hood
  (bind _hood_arrow (Variables|Default|GetHood_arrow))
  (bind _hood_arrow_2 (Variables|Default|GetHood_arrow))
  ;[0.5922 1 0.9929 1 72] Car Hood Anim
  (Utilities|FlowControl|Sequence
    (:then_0
      (bind _open_hood_interpolation_track (Timeline|Open%20Hood%20Interpolation%20Timeline Stop)
        (:Update
          (Transformation|SetRelativeLocationAndRotation _hood_arrow_2 (Math|Vector|Lerp(Vector) (Variables|/Script/Engine.SceneComponent|GetRelativeLocation _hood_arrow_2) "24.000000,-436.000000,102.000000" _open_hood_interpolation_track) (Math|Rotator|Lerp(Rotator) (Variables|/Script/Engine.SceneComponent|GetRelativeRotation _hood_arrow_2) "-45.000000, 0,0.000000" _open_hood_interpolation_track) false false))))
    (:then_1
      (bind _close_hood_interpolation_track (Timeline|Close%20Hood%20Interpolation%20Timeline PlayFromStart)
        (:Update
          (Transformation|SetRelativeLocationAndRotation _hood_arrow (Math|Vector|Lerp(Vector) (Variables|/Script/Engine.SceneComponent|GetRelativeLocation _hood_arrow) "24.000000,-436.000000,102.000000" _close_hood_interpolation_track) (Math|Rotator|Lerp(Rotator) (Variables|/Script/Engine.SceneComponent|GetRelativeRotation _hood_arrow) "0, 0, 0" _close_hood_interpolation_track) false false))))))

(event Custom|Open%20Trunk
  (bind _trunk_arrow (Variables|Default|GetTrunk%20Arrow))
  (bind _trunk_arrow_2 (Variables|Default|GetTrunk%20Arrow))
  ;[0.6856 0.9673 1 1 72] Car Trunk Anim
  (Utilities|FlowControl|Sequence
    (:then_0
      (bind _open_trunk_interpolation_track (Timeline|Timeline_0 Stop)
        (:Update
          (Transformation|SetRelativeLocationAndRotation _trunk_arrow_2 (Math|Vector|Lerp(Vector) (Variables|/Script/Engine.SceneComponent|GetRelativeLocation _trunk_arrow_2) "269.000000,-439.000000,144.000000" _open_trunk_interpolation_track) (Math|Rotator|Lerp(Rotator) (Variables|/Script/Engine.SceneComponent|GetRelativeRotation _trunk_arrow_2) "0, 0, 0" _open_trunk_interpolation_track) false false))))
    (:then_1
      (bind _open_trunk_interpolation_track_2 (Timeline|Open%20Trunk%20Interpolation%20Timeline PlayFromStart)
        (:Update
          (Transformation|SetRelativeLocationAndRotation _trunk_arrow (Math|Vector|Lerp(Vector) (Variables|/Script/Engine.SceneComponent|GetRelativeLocation _trunk_arrow) "269.000000,-439.000000,144.000000" _open_trunk_interpolation_track_2) (Math|Rotator|Lerp(Rotator) (Variables|/Script/Engine.SceneComponent|GetRelativeRotation _trunk_arrow) "45.000000, 0,0.000000" _open_trunk_interpolation_track_2) false false))))))

(event Custom|Close%20Trunk
  (bind _trunk_arrow (Variables|Default|GetTrunk%20Arrow))
  (bind _trunk_arrow_2 (Variables|Default|GetTrunk%20Arrow))
  ;[0.6856 0.9673 1 1 72] Car Trunk Anim
  (Utilities|FlowControl|Sequence
    (:then_0
      (bind _open_trunk_interpolation_track (Timeline|Open%20Trunk%20Interpolation%20Timeline Stop)
        (:Update
          (Transformation|SetRelativeLocationAndRotation _trunk_arrow (Math|Vector|Lerp(Vector) (Variables|/Script/Engine.SceneComponent|GetRelativeLocation _trunk_arrow) "269.000000,-439.000000,144.000000" _open_trunk_interpolation_track) (Math|Rotator|Lerp(Rotator) (Variables|/Script/Engine.SceneComponent|GetRelativeRotation _trunk_arrow) "45.000000, 0,0.000000" _open_trunk_interpolation_track) false false))))
    (:then_1
      (bind _open_trunk_interpolation_track_2 (Timeline|Timeline_0 PlayFromStart)
        (:Update
          (Transformation|SetRelativeLocationAndRotation _trunk_arrow_2 (Math|Vector|Lerp(Vector) (Variables|/Script/Engine.SceneComponent|GetRelativeLocation _trunk_arrow_2) "269.000000,-439.000000,144.000000" _open_trunk_interpolation_track_2) (Math|Rotator|Lerp(Rotator) (Variables|/Script/Engine.SceneComponent|GetRelativeRotation _trunk_arrow_2) "0, 0, 0" _open_trunk_interpolation_track_2) false false))))))

(event Custom|Close%20Front%20Right%20Door
  (bind _front_right_door_pivot_arrow (Variables|Default|GetFront_right_door_pivot_arrow))
  (bind _front_right_door_pivot_arrow_2 (Variables|Default|GetFront_right_door_pivot_arrow))
  ;[0.7144 0.9615 1 1 72] Car Front Right Door Anim
  (Utilities|FlowControl|Sequence
    (:then_0
      (bind _open_front_right_door_interpolation_track (Timeline|Open%20Front%20Right%20Door%20Timeline Stop)
        (:Update
          (Transformation|SetRelativeLocationAndRotation _front_right_door_pivot_arrow (Math|Vector|Lerp(Vector) (Variables|/Script/Engine.SceneComponent|GetRelativeLocation _front_right_door_pivot_arrow) "64.000000,-517.000000,89.000000" _open_front_right_door_interpolation_track) (Math|Rotator|Lerp(Rotator) (Variables|/Script/Engine.SceneComponent|GetRelativeRotation _front_right_door_pivot_arrow) "0.000000,-48.000000,0.000000" _open_front_right_door_interpolation_track) false false))))
    (:then_1
      (bind _close_front_right_door_interpolation_track (Timeline|Close%20Front%20Right%20Door%20Timeline PlayFromStart)
        (:Update
          (Transformation|SetRelativeLocationAndRotation _front_right_door_pivot_arrow_2 (Math|Vector|Lerp(Vector) (Variables|/Script/Engine.SceneComponent|GetRelativeLocation _front_right_door_pivot_arrow_2) "64.000000,-517.000000,89.000000" _close_front_right_door_interpolation_track) (Math|Rotator|Lerp(Rotator) (Variables|/Script/Engine.SceneComponent|GetRelativeRotation _front_right_door_pivot_arrow_2) "0, 0, 0" _close_front_right_door_interpolation_track) false false))))))

(event Custom|Open%20Front%20Right%20Door
  (bind _front_right_door_pivot_arrow (Variables|Default|GetFront_right_door_pivot_arrow))
  (bind _front_right_door_pivot_arrow_2 (Variables|Default|GetFront_right_door_pivot_arrow))
  ;[0.7144 0.9615 1 1 72] Car Front Right Door Anim
  (Utilities|FlowControl|Sequence
    (:then_0
      (bind _close_front_right_door_interpolation_track (Timeline|Close%20Front%20Right%20Door%20Timeline Stop)
        (:Update
          (Transformation|SetRelativeLocationAndRotation _front_right_door_pivot_arrow_2 (Math|Vector|Lerp(Vector) (Variables|/Script/Engine.SceneComponent|GetRelativeLocation _front_right_door_pivot_arrow_2) "64.000000,-517.000000,89.000000" _close_front_right_door_interpolation_track) (Math|Rotator|Lerp(Rotator) (Variables|/Script/Engine.SceneComponent|GetRelativeRotation _front_right_door_pivot_arrow_2) "0, 0, 0" _close_front_right_door_interpolation_track) false false))))
    (:then_1
      (bind _open_front_right_door_interpolation_track (Timeline|Open%20Front%20Right%20Door%20Timeline PlayFromStart)
        (:Update
          (Transformation|SetRelativeLocationAndRotation _front_right_door_pivot_arrow (Math|Vector|Lerp(Vector) (Variables|/Script/Engine.SceneComponent|GetRelativeLocation _front_right_door_pivot_arrow) "64.000000,-517.000000,89.000000" _open_front_right_door_interpolation_track) (Math|Rotator|Lerp(Rotator) (Variables|/Script/Engine.SceneComponent|GetRelativeRotation _front_right_door_pivot_arrow) "0.000000,-48.000000,0.000000" _open_front_right_door_interpolation_track) false false))))))

(event Custom|Open%20Front%20Left%20Door
  (bind _front_left_door_pivot_arrow (Variables|Default|GetFront_left_door_pivot_arrow))
  (bind _front_left_door_pivot_arrow_2 (Variables|Default|GetFront_left_door_pivot_arrow))
  ;[0.6928 1 0.9815 1 72] Car Front Left Door Anim
  (Utilities|FlowControl|Sequence
    (:then_0
      (bind _close_front_left_door_interpolation_track (Timeline|Close%20Front%20Left%20Door%20Timeline Stop)
        (:Update
          (Transformation|SetRelativeLocationAndRotation _front_left_door_pivot_arrow_2 (Math|Vector|Lerp(Vector) (Variables|/Script/Engine.SceneComponent|GetRelativeLocation _front_left_door_pivot_arrow_2) "64.000000,-360.000000,89.000000" _close_front_left_door_interpolation_track) (Math|Rotator|Lerp(Rotator) (Variables|/Script/Engine.SceneComponent|GetRelativeRotation _front_left_door_pivot_arrow_2) "0, 0, 0" _close_front_left_door_interpolation_track) false false))))
    (:then_1
      (bind _open_front_left_door_interpolation_track (Timeline|Open%20Front%20Left%20Door%20Timeline PlayFromStart)
        (:Update
          (Transformation|SetRelativeLocationAndRotation _front_left_door_pivot_arrow (Math|Vector|Lerp(Vector) (Variables|/Script/Engine.SceneComponent|GetRelativeLocation _front_left_door_pivot_arrow) "64.000000,-360.000000,89.000000" _open_front_left_door_interpolation_track) (Math|Rotator|Lerp(Rotator) (Variables|/Script/Engine.SceneComponent|GetRelativeRotation _front_left_door_pivot_arrow) "0.000000,48.000000,0.000000" _open_front_left_door_interpolation_track) false false))))))

(event Custom|Open%20Rear%20Right%20Door
  (bind _rear_right_door_pivot_arrow (Variables|Default|GetRear_right_door_pivot_arrow))
  (bind _rear_right_door_pivot_arrow_2 (Variables|Default|GetRear_right_door_pivot_arrow))
  ;[0.614 1 0.9801 1 72] Car Rear Right Door Anim
  (Utilities|FlowControl|Sequence
    (:then_0
      (bind _close_front_left_door_interpolation_track (Timeline|Timeline_4 Stop)
        (:Update
          (Transformation|SetRelativeLocationAndRotation _rear_right_door_pivot_arrow_2 (Math|Vector|Lerp(Vector) (Variables|/Script/Engine.SceneComponent|GetRelativeLocation _rear_right_door_pivot_arrow_2) "166.000000,-513.000000,96.000000" _close_front_left_door_interpolation_track) (Math|Rotator|Lerp(Rotator) (Variables|/Script/Engine.SceneComponent|GetRelativeRotation _rear_right_door_pivot_arrow_2) "0, 0, 0" _close_front_left_door_interpolation_track) false false))))
    (:then_1
      (bind _open_front_left_door_interpolation_track (Timeline|Timeline_3 PlayFromStart)
        (:Update
          (Transformation|SetRelativeLocationAndRotation _rear_right_door_pivot_arrow (Math|Vector|Lerp(Vector) (Variables|/Script/Engine.SceneComponent|GetRelativeLocation _rear_right_door_pivot_arrow) "166.000000,-513.000000,96.000000" _open_front_left_door_interpolation_track) (Math|Rotator|Lerp(Rotator) (Variables|/Script/Engine.SceneComponent|GetRelativeRotation _rear_right_door_pivot_arrow) "0.000000,-48.000000,0.000000" _open_front_left_door_interpolation_track) false false))))))

(event EventBeginPlay
  ;[0.418 1 0.9588 1 72] Integrating CPP_VehicleExteriorData <-> Widget_VehicleExteriorData, Calling necessary animations according to CPP_Instance variable inputs
  (bind _returnvalue (Actor|GetActorOfClass "/Game/ConsoleHMI/Blueprints/InstrumentCluster_CppBP.InstrumentCluster_CppBP_C"))
  (bind _asinstrument_cluster_cpp_bp (Utilities|Casting|CastToInstrumentCluster_CppBP _returnvalue)))

(event EventTick
  (params (DeltaSeconds :type Float%20%28single-precision%29))
  ;[0.418 1 0.9588 1 72] Integrating CPP_VehicleExteriorData <-> Widget_VehicleExteriorData, Calling necessary animations according to CPP_Instance variable inputs
  (Utilities|FlowControl|Sequence
    (:then_0
      (if (Variables|/Script/ConsoleHMI.InstrumentCluster_Cpp|GetVehicleHoodState (stale EventBeginPlay _asinstrument_cluster_cpp_bp))
        (Utilities|FlowControl|DoOnce false :!label _label
          (:Completed
            (CallFunction|OpenHood)
            (goto _label_2 Reset)))
        (else
          (Utilities|FlowControl|DoOnce false :!label _label_2
            (:Completed
              (CallFunction|CloseHood)
              (goto _label Reset))))))
    (:then_1
      (if (Variables|/Script/ConsoleHMI.InstrumentCluster_Cpp|GetVehicleSunRoofState (stale EventBeginPlay _asinstrument_cluster_cpp_bp))
        (Utilities|FlowControl|DoOnce false :!label _label_3
          (:Completed
            (CallFunction|OpenSunRoof)
            (goto _label_4 Reset)))
        (else
          (Utilities|FlowControl|DoOnce false :!label _label_4
            (:Completed
              (CallFunction|CloseSunRoof)
              (goto _label_3 Reset))))))
    (:then_2
      (if (Variables|/Script/ConsoleHMI.InstrumentCluster_Cpp|GetVehicleFrontLeftDoorState (stale EventBeginPlay _asinstrument_cluster_cpp_bp))
        (Utilities|FlowControl|DoOnce false :!label _label_5
          (:Completed
            (CallFunction|OpenFrontLeftDoor)
            (goto _label_6 Reset)))
        (else
          (Utilities|FlowControl|DoOnce false :!label _label_6
            (:Completed
              (CallFunction|CloseFrontLeftDoor)
              (goto _label_5 Reset))))))
    (:then_3
      (if (Variables|/Script/ConsoleHMI.InstrumentCluster_Cpp|GetVehicleFrontRightDoorState (stale EventBeginPlay _asinstrument_cluster_cpp_bp))
        (Utilities|FlowControl|DoOnce false :!label _label_7
          (:Completed
            (CallFunction|OpenFrontRightDoor)
            (goto _label_8 Reset)))
        (else
          (Utilities|FlowControl|DoOnce false :!label _label_8
            (:Completed
              (CallFunction|CloseFrontRightDoor)
              (goto _label_7 Reset))))))
    (:then_4
      (if (Variables|/Script/ConsoleHMI.InstrumentCluster_Cpp|GetVehicleRearLeftDoorState (stale EventBeginPlay _asinstrument_cluster_cpp_bp))
        (Utilities|FlowControl|DoOnce false :!label _label_9
          (:Completed
            (CallFunction|OpenRearLeftDoor)
            (goto _label_10 Reset)))
        (else
          (Utilities|FlowControl|DoOnce false :!label _label_10
            (:Completed
              (CallFunction|CloseRearLeftDoor)
              (goto _label_9 Reset))))))
    (:then_5
      (if (Variables|/Script/ConsoleHMI.InstrumentCluster_Cpp|GetVehicleRearRightDoorState (stale EventBeginPlay _asinstrument_cluster_cpp_bp))
        (Utilities|FlowControl|DoOnce false :!label _label_11
          (:Completed
            (CallFunction|OpenRearRightDoor)
            (goto _label_12 Reset)))
        (else
          (Utilities|FlowControl|DoOnce false :!label _label_12
            (:Completed
              (CallFunction|CloseRearRightDoor)
              (goto _label_11 Reset))))))
    (:then_6
      (if (Variables|/Script/ConsoleHMI.InstrumentCluster_Cpp|GetVehicleTrunkState (stale EventBeginPlay _asinstrument_cluster_cpp_bp))
        (Utilities|FlowControl|DoOnce false :!label _label_13
          (:Completed
            (CallFunction|OpenTrunk)
            (goto _label_14 Reset)))
        (else
          (Utilities|FlowControl|DoOnce false :!label _label_14
            (:Completed
              (CallFunction|CloseTrunk)
              (goto _label_13 Reset))))))))

(fn ConstructionScript)